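; MagicianController is a player controller that turns Enhanced Input actions into look and movement for the controlled magician pawn.
; BeginPlay registers the IMC_Magician mapping context with the local player's Enhanced Input subsystem.
; The rotate action adds yaw and pitch input to the controller.
; The move action drives the pawn along right and forward vectors built only from control yaw, keeping movement level regardless of camera pitch.
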(event `self.ReceiveBeginPlay`
  (`EnhancedInputSubsystemInterface.AddMappingContext` (subsystem `EnhancedInputLocalPlayerSubsystem`) "/Game/MyAsset/Input/IMC_Magician.IMC_Magician" 0 (struct)))

(event `EnhancedInput|/Game/MyAsset/Input/IA_RotateMagician`
  (params (ActionValue :type "Vector2D Structure") (ElapsedSeconds :type "Float (double-precision)") (TriggeredSeconds :type "Float (double-precision)") (InputAction :type "InputAction Object Reference" :default "/Game/MyAsset/Input/IA_RotateMagician.IA_RotateMagician"))
  (:`Triggered`
    (`self.AddYawInput` ActionValue_X)
    (`self.AddPitchInput` ActionValue_Y)))

(event `EnhancedInput|/Game/MyAsset/Input/IA_MoveMagician`
  (params (ActionValue :type "Vector2D Structure") (ElapsedSeconds :type "Float (double-precision)") (TriggeredSeconds :type "Float (double-precision)") (InputAction :type "InputAction Object Reference" :default "/Game/MyAsset/Input/IA_MoveMagician.IA_MoveMagician"))
  (bind (_returnvalue_roll _returnvalue_pitch _returnvalue_yaw) (`KismetMathLibrary.BreakRotator` (`self.GetControlRotation`)))
  (bind (_returnvalue_roll_2 _returnvalue_pitch_2 _returnvalue_yaw_2) (`KismetMathLibrary.BreakRotator` (`self.GetControlRotation`)))
  (:`Triggered`
    (`Pawn.AddMovementInput` (`self.K2_GetPawn`) (`KismetMathLibrary.GetRightVector` (`KismetMathLibrary.MakeRotator` 0.0 0.0 _returnvalue_yaw_2)) ActionValue_X false)
    (`Pawn.AddMovementInput` (`self.K2_GetPawn`) (`KismetMathLibrary.GetForwardVector` (`KismetMathLibrary.MakeRotator` 0.0 0.0 _returnvalue_yaw)) ActionValue_Y false)))

(fn `UserConstructionScript`)